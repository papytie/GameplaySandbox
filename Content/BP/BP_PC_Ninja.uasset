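; BP_PC_Ninja is a playable platformer character that moves, jumps and dashes through Enhanced Input.
; BeginPlay adds the platformer mapping context, and move input is applied along control-rotation axes, X forward and Y right.
; Dash is a swept location offset along control yaw, repeated each time the action triggers, rather than a velocity impulse.
; Jump and dash also set IsJumping and IsDashing flags, cleared when each input completes.
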(event `self.ReceiveBeginPlay`
  (bind _asplayer_controller (cast `PlayerController` (`self.GetController`)))
  (bind _returnvalue (pcsubsystem `EnhancedInputLocalPlayerSubsystem` _asplayer_controller))
  (`/Engine/EditorBlueprintResources/StandardMacros.IsValid` _returnvalue
    (:`Is Valid`
      (`EnhancedInputSubsystemInterface.AddMappingContext` _returnvalue "/Game/BP/Imputs/IMC_PlatformerCharacter.IMC_PlatformerCharacter" 0 (struct)))))

(event `EnhancedInput|/Game/BP/Imputs/IA_Move`
  (params (ActionValue :type "Vector2D Structure") (ElapsedSeconds :type "Float (double-precision)") (TriggeredSeconds :type "Float (double-precision)") (InputAction :type "InputAction Object Reference" :default "/Game/BP/Imputs/IA_Move.IA_Move"))
  (bind (_returnvalue_roll _returnvalue_pitch _returnvalue_yaw) (`KismetMathLibrary.BreakRotator` (`self.GetControlRotation`)))
  (bind (_returnvalue_roll_2 _returnvalue_pitch_2 _returnvalue_yaw_2) (`KismetMathLibrary.BreakRotator` (`self.GetControlRotation`)))
  (:`Triggered`
    (bind _output_get (set `self.Action Value X` ActionValue_X :!label _label))
    (bind _output_get_2 (set `self.Action Value Y` ActionValue_Y))
    (`self.AddMovementInput` (`KismetMathLibrary.GetRightVector` (`KismetMathLibrary.MakeRotator` _returnvalue_roll 0.0 _returnvalue_yaw)) _output_get_2)
    (`self.AddMovementInput` (`KismetMathLibrary.GetForwardVector` (`KismetMathLibrary.MakeRotator` 0.0 0.0 _returnvalue_yaw_2)) _output_get))
  (:`Completed`
    (goto _label)))

(event `EnhancedInput|/Game/BP/Imputs/IA_Jump`
  (params (ActionValue :type Boolean) (ElapsedSeconds :type "Float (double-precision)") (TriggeredSeconds :type "Float (double-precision)") (InputAction :type "InputAction Object Reference" :default "/Game/BP/Imputs/IA_Jump.IA_Jump"))
  (:`Started`
    (`self.Jump`)
    (set `self.isJumping` true))
  (:`Completed`
    (set `self.isJumping` false)))

(event `EnhancedInput|/Game/BP/Imputs/IA_Dash`
  (params (ActionValue :type Boolean) (ElapsedSeconds :type "Float (double-precision)") (TriggeredSeconds :type "Float (double-precision)") (InputAction :type "InputAction Object Reference" :default "/Game/BP/Imputs/IA_Dash.IA_Dash"))
  (bind (_returnvalue_roll _returnvalue_pitch _returnvalue_yaw) (`KismetMathLibrary.BreakRotator` (`self.GetControlRotation`)))
  (:`Triggered`
    (set `self.isDashing` true)
    (`self.K2_SetActorLocation` (+ (`self.K2_GetActorLocation`) (* (`KismetMathLibrary.GetForwardVector` (`KismetMathLibrary.MakeRotator` 0.0 0.0 _returnvalue_yaw)) 100.0)) true))
  (:`Completed`
    (set `self.isDashing` false)))

(fn `UserConstructionScript`)